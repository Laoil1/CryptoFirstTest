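; BP_Cryptid is a parent Blueprint for cryptids that the player photographs to discover.
; When shot, it passes its Cryptid enum and the render target to the first player's BP_PSCrypto player state, which stores the photo and marks that cryptid discovered.
; The construction script calls its parent, then derives ObjectName from the Cryptid enum, so the name follows the selected type.
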(event EventShootedObject
  (params (RenderTarget :type Texture%20Render%20Target%202D%20Object%20Reference))
  (bind _returnvalue (Game|GetPlayerController 0))
  (bind _playerstate (Variables|/Script/Engine.Controller|GetPlayerState _returnvalue))
  (bind _asbp_pscrypto (Utilities|Casting|CastToBP_PSCrypto _playerstate))
  (Default|SetPhotoonCryptid _asbp_pscrypto (Variables|Default|GetCryptid) RenderTarget)
  (Default|DiscoverCryptid _asbp_pscrypto (Variables|Default|GetCryptid)))

(fn ConstructionScript
  (|CallParentFunction)
  (Variables|Default|SetObjectName (Utilities|String|EnumtoString (Variables|Default|GetCryptid))))