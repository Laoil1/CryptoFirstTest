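; Base interactable actor with an empty Interact event and InteractFunction, presumably for child Blueprints to override.
; Its Sphere sets itself as the FirstPersonCharacter's InteractObject on overlap and clears that reference when the character leaves.
; SetToDestroy hides the actor and flags it, deferring destruction until the character's overlap ends.
; The construction script caches the first BP_UISetter found in the level.
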(event OnComponentEndOverlap(Sphere)
  (params (OverlappedComponent :type Primitive%20Component%20Object%20Reference) (OtherActor :type Actor%20Object%20Reference) (OtherComp :type Primitive%20Component%20Object%20Reference) (OtherBodyIndex :type Integer))
  (bind _asfirst_person_character (Utilities|Casting|CastToFirstPersonCharacter OtherActor))
  (Variables|/Game/Blueprints/FirstPersonCharacter.FirstPersonCharacter_C|SetInteractObject _asfirst_person_character 0)
  (if (Variables|Default|GetToDestroy)
    (Actor|DestroyActor)))

(event OnComponentBeginOverlap(Sphere)
  (params (OverlappedComponent :type Primitive%20Component%20Object%20Reference) (OtherActor :type Actor%20Object%20Reference) (OtherComp :type Primitive%20Component%20Object%20Reference) (OtherBodyIndex :type Integer) (bFromSweep :type Boolean) (SweepResult :type Hit%20Result%20Structure%20%28by%20ref%29))
  (Variables|/Game/Blueprints/FirstPersonCharacter.FirstPersonCharacter_C|SetInteractObject (.AsFirst%20Person%20Character (Utilities|Casting|CastToFirstPersonCharacter OtherActor)) self))

(event Custom|Interact
  (params (player :type First%20Person%20Character%20Object%20Reference)))

(event Custom|SetToDestroy
  (Variables|Default|SetToDestroy true)
  (Rendering|SetActorHiddenInGame true))

(fn ConstructionScript
  (bind _outactors (Actor|GetAllActorsOfClass "/Game/Blueprints/BP_UISetter.BP_UISetter_C"))
  (Variables|Default|SetUI_Setter (Utilities|Array|Get(acopy) _outactors)))

(fn InteractFunction
  (return))