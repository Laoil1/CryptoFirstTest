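; BP_Clue is an interactable clue that reveals encyclopedia information about a specific cryptid.
; On Interact, three flags choose which facts it reveals for ConcernedCryptid: location, weather and time of apparition.
; Each enabled flag calls the matching discover function on the first player's BP_PSCrypto player state, then plays a notification message through UISetter.
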(event EventInteract
  ;[0.1566 1 0.07239] SetInformationsAtEncyclopédia
  (Utilities|FlowControl|Sequence
    (:then_0
      (if (Variables|Default|GetdiscoverPosition)
        (Default|DiscoverPosition (.AsBP%20PSCrypto (Utilities|Casting|CastToBP_PSCrypto (Variables|/Script/Engine.Controller|GetPlayerState (Game|GetPlayerController 0)))) (Variables|Default|GetConcernedCryptid))
        (Default|PlayUpdateAnimation (Variables|Default|GetUI_Setter) "You Found information about a Cryptid Location")))
    (:then_1
      (if (Variables|Default|GetdiscoverMeteo)
        (Default|DiscoverMeteo (.AsBP%20PSCrypto (Utilities|Casting|CastToBP_PSCrypto (Variables|/Script/Engine.Controller|GetPlayerState (Game|GetPlayerController 0)))) (Variables|Default|GetConcernedCryptid))
        (Default|PlayUpdateAnimation (Variables|Default|GetUI_Setter) "You Found information about a Cryptid weather ")))
    (:then_2
      (if (Variables|Default|GetdiscoverTime)
        (Default|DiscoverTime (.AsBP%20PSCrypto (Utilities|Casting|CastToBP_PSCrypto (Variables|/Script/Engine.Controller|GetPlayerState (Game|GetPlayerController 0)))) (Variables|Default|GetConcernedCryptid))
        (Default|PlayUpdateAnimation (Variables|Default|GetUI_Setter) "You Found information about a Cryptid Time Of Apparition ")))))

(fn ConstructionScript
  (|CallParentFunction))